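; VR motion logger that records HMD, torso tracker and platform tracker data, saving each series to text files on EndPlay.
; BeginPlay sets a floor origin and derives the fixed tracker-to-platform transform from preset initial measurements.
; Each Tick reads the devices and re-derives the initial-HMD-to-platform basis from the platform tracker.
; Chained matrix multiplies and inverses then yield head and torso poses relative to platform and each other, with velocity and acceleration.
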(event Custom|Cal_Transform_T_wrt_H
  (params (DeltaSeconds :type Float%20%28single-precision%29))
  ;[1 1 1] calculating Data of Torso with respect to Head
  (bind _returnvalue (Class|TransformationMatrixLib|TransformationMatrixInverse (Variables|Default|GetTransformation_H_wrt_T)))
  (bind _output_get (Variables|Default|SetTransformation_T_wrt_H _returnvalue))
  (bind _returnvalue_2 (Class|TransformationMatrixLib|TransformationMatrixPositionExtract _output_get))
  (bind _returnvalue_3 (Class|TransformationMatrixLib|TransformationMatrixRotationRPYExtract _output_get))
  (bind _gettrackerdatafunc_out (CallFunction|CalVelandAcc _returnvalue_2 _returnvalue_3 DeltaSeconds))
  (bind _output_get_2 (Variables|Default|SetData_Torso_wrt_Head _gettrackerdatafunc_out))
  (Utilities|Array|Add (Variables|Default|GetFinal_DataTorso_wrt_Head) _output_get_2))

(event Custom|SaveData2
  (params (EndPLay%20Reason :type EEndPlayReason%20Enum :default "Destroyed"))
  ;[1 1 1] Tracker Platform B with respect to HMD(initial0)
  ;;[1 1 1] Save Data to Text
  (CallFunction|SaveTrackerDatatxt (Variables|Default|GetFinal_TR_PlatformB_TrackerDataStruct) (Variables|Default|GetFolderName) (Utilities|GetObjectName (Variables|Default|GetTR_PlatformB)) (Variables|Default|GetIsFileOverWriting)))

(event Custom|Save_Data_H_wrt_T
  (params (EndPlayReason :type EEndPlayReason%20Enum :default "Destroyed"))
  ;[1 1 1] Calculating data of Head with respect to torso
  ;;[1 1 1] Save Data to Text
  (CallFunction|SaveTrackerDatatxt (Variables|Default|GetFinal_DataHead_wrt_Torso) (Variables|Default|GetFolderName) "Data Head wrt Torso" (Variables|Default|GetIsFileOverWriting)))

(event Custom|Cal_Transform_H_wrt_P
  (params (DeltaSeconds :type Float%20%28single-precision%29))
  ;[1 1 1] Calculating data of head with respect to platform
  (bind _returnvalue (Class|TransformationMatrixLib|TransformationMatrixMultiply (Variables|Default|GetTransformation_H0_wrt_P) (Variables|Default|GetTransformation_H_wrt_H0)))
  (bind _output_get (Variables|Default|SetTransformation_H_wrt_P _returnvalue))
  (bind _returnvalue_2 (Class|TransformationMatrixLib|TransformationMatrixPositionExtract _output_get))
  (bind _returnvalue_3 (Class|TransformationMatrixLib|TransformationMatrixRotationRPYExtract _output_get))
  (bind _gettrackerdatafunc_out (CallFunction|CalVelandAcc _returnvalue_2 _returnvalue_3 DeltaSeconds))
  (bind _output_get_2 (Variables|Default|SetData_Head_wrt_Platform _gettrackerdatafunc_out))
  (Utilities|Array|Add (Variables|Default|GetFinal_Data_Head_wrt_Platform) _output_get_2))

(event Custom|Save_Data_H_wrt_P
  (params (EndPlayReason :type EEndPlayReason%20Enum :default "Destroyed"))
  ;[1 1 1] Calculating data of head with respect to platform
  ;;[1 1 1] Save Data to Text
  (CallFunction|SaveTrackerDatatxt (Variables|Default|GetFinal_Data_Head_wrt_Platform) (Variables|Default|GetFolderName) "Data Head wrt Platform" (Variables|Default|GetIsFileOverWriting)))

(event Custom|Save_Data_T_wrt_H
  (params (EndPlayReason :type EEndPlayReason%20Enum :default "Destroyed"))
  ;[1 1 1] calculating Data of Torso with respect to Head
  ;;[1 1 1] Save Data to Text
  (CallFunction|SaveTrackerDatatxt (Variables|Default|GetFinal_DataTorso_wrt_Head) (Variables|Default|GetFolderName) "Data Torso wrt Head" (Variables|Default|GetIsFileOverWriting)))

(event Custom|Cal_Transform_T_wrt_P
  (params (DeltaSeconds :type Float%20%28single-precision%29))
  ;[1 1 1] Calculating data of Torso with respect to platform
  (bind _returnvalue (Class|TransformationMatrixLib|TransformationMatrixMultiply (Variables|Default|GetTransformation_H0_wrt_P) (Variables|Default|GetTransformation_T_wrt_H0)))
  (bind _output_get (Variables|Default|SetTransformation_T_wrt_P _returnvalue))
  (bind _returnvalue_2 (Class|TransformationMatrixLib|TransformationMatrixPositionExtract _output_get))
  (bind _returnvalue_3 (Class|TransformationMatrixLib|TransformationMatrixRotationRPYExtract _output_get))
  (bind _gettrackerdatafunc_out (CallFunction|CalVelandAcc _returnvalue_2 _returnvalue_3 DeltaSeconds))
  (bind _output_get_2 (Variables|Default|SetData_Torso_wrt_Platform _gettrackerdatafunc_out))
  (Utilities|Array|Add (Variables|Default|GetFinal_DataTorso_wrt_Platform) _output_get_2))

(event Custom|Save_Data_T_wrt_P
  (params (EndPlayReason :type EEndPlayReason%20Enum :default "Destroyed"))
  ;[1 1 1] Calculating data of Torso with respect to platform
  ;;[1 1 1] Save Data to Text
  (CallFunction|SaveTrackerDatatxt (Variables|Default|GetFinal_DataTorso_wrt_Platform) (Variables|Default|GetFolderName) "Data Torso wrt Platform" (Variables|Default|GetIsFileOverWriting)))

(event Custom|Initial%20Measurements
  ;[1 1 1] Measurement with Initial settings
  (bind _returnvalue (Class|TransformationMatrixLib|TransformationMatrix (Variables|Default|GetInitialRotMeasurement_B_wrt_H0) (Variables|Default|GetInitialPosMeasurement_B_wrt_H0)))
  (Variables|Default|SetInitialTransformation_B_wrt_H0 _returnvalue)
  (bind _returnvalue_2 (Class|TransformationMatrixLib|TransformationMatrix (Variables|Default|GetInitialRotMeasurement_P_wrt_H0) (Variables|Default|GetInitialPosMeasurement_P_wrt_H0)))
  (Variables|Default|SetInitialTransformation_P_wrt_H0 _returnvalue_2)
  ;;[1 1 1] Calucation of Transformation of B with respect to P
  (bind _returnvalue_3 (Class|TransformationMatrixLib|TransformationMatrixInverse (Variables|Default|GetInitialTransformation_P_wrt_H0)))
  (bind _returnvalue_4 (Class|TransformationMatrixLib|TransformationMatrixMultiply _returnvalue_3 (Variables|Default|GetInitialTransformation_B_wrt_H0)))
  (Variables|Default|SetTransformation_B_wrt_P _returnvalue_4))

(event Custom|Cal%20Transform%20H0%20wrt%20P
  ;[1 1 1] Calculation Transformation of H0 with respect to P (Basis change)
  (bind _returnvalue (Class|TransformationMatrixLib|TransformationMatrixInverse (Variables|Default|GetTransformation_B_wrt_H0)))
  (bind _returnvalue_2 (Class|TransformationMatrixLib|TransformationMatrixMultiply (Variables|Default|GetTransformation_B_wrt_P) _returnvalue))
  (Variables|Default|SetTransformation_H0_wrt_P _returnvalue_2))

(event Custom|ExtractTrackerData3
  (params (DeltaSeconds :type Float%20%28single-precision%29))
  ;[1 1 1] Tracker Torso data with respect to HMD(initial0)
  ;;[1 1 1] Extract data from Tracker of Torso (Vive 2.0)
  (bind (_gettrackerdatafunc_out _transformationmatrix_wrt_base) (CallFunction|GetTrackerData (Variables|Default|GetTR_Torso2_0) DeltaSeconds))
  (Variables|Default|SetTransformation_T_wrt_H0 _transformationmatrix_wrt_base)
  (bind _output_get (Variables|Default|SetTR_Torso2_0_TrackerDataStruct _gettrackerdatafunc_out))
  (Utilities|Array|Add (Variables|Default|GetFinal_TR_Torso2_0_TrackerDataStruct) _output_get))

(event Custom|Cal_Transform_H_wrt_T
  (params (DeltaSeconds :type Float%20%28single-precision%29))
  ;[1 1 1] Calculating data of Head with respect to torso
  (bind _returnvalue (Class|TransformationMatrixLib|TransformationMatrixInverse (Variables|Default|GetTransformation_T_wrt_H0)))
  (bind _returnvalue_2 (Class|TransformationMatrixLib|TransformationMatrixMultiply _returnvalue (Variables|Default|GetTransformation_H_wrt_H0)))
  (bind _output_get (Variables|Default|SetTransformation_H_wrt_T _returnvalue_2))
  (bind _returnvalue_3 (Class|TransformationMatrixLib|TransformationMatrixPositionExtract _output_get))
  (bind _returnvalue_4 (Class|TransformationMatrixLib|TransformationMatrixRotationRPYExtract _output_get))
  (bind _gettrackerdatafunc_out (CallFunction|CalVelandAcc _returnvalue_3 _returnvalue_4 DeltaSeconds))
  (bind _output_get_2 (Variables|Default|SetData_Head_wrt_Torso _gettrackerdatafunc_out))
  (Utilities|Array|Add (Variables|Default|GetFinal_DataHead_wrt_Torso) _output_get_2))

(event Custom|SaveData3
  (params (EndPLayReason :type EEndPlayReason%20Enum :default "Destroyed"))
  ;[1 1 1] Tracker Torso data with respect to HMD(initial0)
  ;;[1 1 1] Save Data to txt
  (CallFunction|SaveTrackerDatatxt (Variables|Default|GetFinal_TR_Torso2_0_TrackerDataStruct) (Variables|Default|GetFolderName) (Utilities|GetObjectName (Variables|Default|GetTR_Torso2_0)) (Variables|Default|GetIsFileOverWriting)))

(event Custom|ExtractHMDData
  (params (DeltaSeconds :type Float%20%28single-precision%29))
  ;[1 1 1] HMD Data with respect to HMD(initial0)
  ;;[1 1 1] Extract Data from HMD using steam VR function
  (bind (_outfunctrackerdatastruct _transformationmatrix) (CallFunction|ExtractTrackerData (Variables|Default|GetShowHMDMesh) (Variables|Default|GetHMD) DeltaSeconds "HMD"))
  (Variables|Default|SetTransformation_H_wrt_H0 _transformationmatrix)
  (bind _output_get (Variables|Default|SetHMD_TrackerDataStruct _outfunctrackerdatastruct))
  (Utilities|Array|Add (Variables|Default|GetFinal_HMD_TrackerDataStruct) _output_get))

(event Custom|SaveHMDData
  (params (EndPlayReason :type EEndPlayReason%20Enum :default "Destroyed"))
  ;[1 1 1] HMD Data with respect to HMD(initial0)
  ;;[1 1 1] Save HMD data to txt
  (CallFunction|SaveTrackerDatatxt (Variables|Default|GetFinal_HMD_TrackerDataStruct) (Variables|Default|GetFolderName) "HMD" (Variables|Default|GetIsFileOverWriting)))

(event Custom|ExtractTrackerData2
  (params (DeltaSeconds :type Float%20%28single-precision%29))
  ;[1 1 1] Tracker Platform B with respect to HMD(initial0)
  ;;[1 1 1] Extract data from Tracker and set the static mesh
  (bind (_gettrackerdatafunc_out _transformationmatrix_wrt_base) (CallFunction|GetTrackerData (Variables|Default|GetTR_PlatformB) DeltaSeconds))
  (Variables|Default|SetTransformation_B_wrt_H0 _transformationmatrix_wrt_base)
  (bind _output_get (Variables|Default|SetTR_PlatformB_TrackerDataStruct _gettrackerdatafunc_out))
  (Utilities|Array|Add (Variables|Default|GetFinal_TR_PlatformB_TrackerDataStruct) _output_get))

(event EventBeginPlay
  ;[1 1 1] Set up a Standing Camera for Steam VR
  (Class|HeadMountedDisplayFunctionLibrary|SetTrackingOrigin "Floor")
  ;[1 1 1] Run Initial calibration
  (CallFunction|InitialMeasurements))

(event EventTick
  (params (DeltaSeconds :type Float%20%28single-precision%29))
  (CallFunction|ExtractTrackerData2 DeltaSeconds)
  (CallFunction|ExtractTrackerData3 DeltaSeconds)
  (CallFunction|ExtractHMDData DeltaSeconds)
  (CallFunction|CalTransformH0WrtP)
  (CallFunction|CalTransformHWrtP DeltaSeconds)
  (CallFunction|CalTransformTWrtP DeltaSeconds)
  (CallFunction|CalTransformHWrtT DeltaSeconds)
  (CallFunction|CalTransformTWrtH DeltaSeconds))

(event EventEndPlay
  (params (EndPlayReason :type EEndPlayReason%20Enum :default "Destroyed"))
  (CallFunction|SaveData2 EndPlayReason)
  (CallFunction|SaveData3 EndPlayReason)
  (CallFunction|SaveHMDData EndPlayReason)
  (CallFunction|SaveDataHWrtP EndPlayReason)
  (CallFunction|SaveDataTWrtP EndPlayReason)
  (CallFunction|SaveDataHWrtT EndPlayReason)
  (CallFunction|SaveDataTWrtH EndPlayReason))

(fn ConstructionScript)