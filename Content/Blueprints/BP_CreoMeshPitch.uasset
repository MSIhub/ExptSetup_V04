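; Creo mesh pitch actor that plays a recorded motion on the player pawn as a visual cue, started by the S key.
; The PitchMeshData timeline supplies position and orientation, remapped from Creo to Unreal axes, with position also transformed by RotationMesh and raised by ZOffset.
; Levels without "NoMotion" in their name also start the pawn sending data to SP7.
; When the timeline finishes, the pawn's SP platform communication component stops ticking.
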(event Custom|Play
  (bind _returnvalue (Game|Player|GetPlayerPawn 0))
  ;[1 1 1] Moving the creo mesh, visual cue
  ;;[1 1 1] If the level name has NoMotion in it, d not send data to SP7
  (bind _returnvalue_2 (Game|GetCurrentLevelName true))
  (if (Class|VictoryBPFunctionLibrary|HasSubstring _returnvalue_2 "NoMotion" "IgnoreCase" "FromStart")
    (bind (_direction _position _orientation) (Timeline|PitchMeshData Play)
      (:Update
        ;;[1 1 1] Transformation for the visual mesh rotations
        (bind _returnvalue_3 (Class|TransformationMatrixLib|TransformationMatrix (Math|Rotator|MakeRotator (* (.y _orientation) -1.0) (.z _orientation) (* (.x _orientation) -1.0)) (Math|Vector|MakeVector (.y _position) (* (.z _position) -1.0) (* (.x _position) -1.0))))
        (bind _returnvalue_4 (Class|TransformationMatrixLib|TransformationMatrix (Variables|Default|GetRotationMesh) "0, 0, 0"))
        (bind _returnvalue_5 (Class|TransformationMatrixLib|TransformationMatrixMultiply _returnvalue_4 _returnvalue_3))
        (bind _returnvalue_6 (Class|TransformationMatrixLib|TransformationMatrixPositionExtract _returnvalue_5))
        (Transformation|SetActorLocationAndRotation (Game|Player|GetPlayerPawn 0) (Math|Vector|MakeVector (.x _returnvalue_6) (.y _returnvalue_6) (+ (.z _returnvalue_6) (Variables|Default|GetZ_Offset))) (Math|Rotator|MakeRotator (* (.Yaw (Math|Rotator|BreakRotator (Math|Rotator|MakeRotator (* (.y _orientation) -1.0) (.z _orientation) (* (.x _orientation) -1.0)))) -1.0) (.Roll (Math|Rotator|BreakRotator (Math|Rotator|MakeRotator (* (.y _orientation) -1.0) (.z _orientation) (* (.x _orientation) -1.0)))) (* (.Pitch (Math|Rotator|BreakRotator (Math|Rotator|MakeRotator (* (.y _orientation) -1.0) (.z _orientation) (* (.x _orientation) -1.0)))) -1.0))))
      (:Finished
        ;;[1 1 1] Send Data to SP7
        (Components|Tick|SetComponentTickEnabled (Actor|GetComponentbyClass _returnvalue "/SPPlatformCommunication/BP_SPPlatformCommunicationComponent.BP_SPPlatformCommunicationComponent_C") false)))
    (else
      (bind _asbp_pawn_following_mesh (Utilities|Casting|CastToBP_PawnFollowingMesh _returnvalue))
      (Default|SendDatatoSP7 _asbp_pawn_following_mesh)
      (Timeline|PitchMeshData Play))))

(event Input|KeyboardEvents|S
  (params (Key :type Key%20Structure))
  ;[1 1 1] Moving the creo mesh, visual cue
  (:Pressed
    (CallFunction|Play)))

(fn ConstructionScript)