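; Startup selector that sets the order of roll, pitch and yaw levels, with and without motion, after training.
; Keys 1–6 pass level lists to StartCustomlevelOrder, which appends another Credits and stores them in GI_GameInstanceCustom.
; Despite six permutation comments, the lists form only two distinct orders, roll-first or pitch-first, both with yaw last.
; Space shows a loading message and, after a delay, calls NextLevel if an order is set.
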(event EventBeginPlay
  (bind _asgi_game_instance_custom (Utilities|Casting|CastToGI_GameInstanceCustom (Game|GetGameInstance)))
  (Variables|Default|SetGI _asgi_game_instance_custom))

(event Input|KeyboardEvents|SpaceBar
  (params (Key :type Key%20Structure))
  (bind _gi (Variables|Default|GetGI))
  ;[1 1 1] Press S for starting the game
  (:Pressed
    (if (> (Utilities|Array|Length (Variables|/Game/Blueprints/GI_GameInstanceCustom.GI_GameInstanceCustom_C|GetLevelsOrder _gi)) 0)
      (Rendering|Components|TextRender|SetText (Variables|Default|GetTextRender) (Utilities|Text|MakeLiteralText "Please wait, loading......"))
      (Utilities|FlowControl|Delay 1.0)
      (Default|NextLevel _gi))))

(event Input|KeyboardEvents|4
  (params (Key :type Key%20Structure))
  ;[1 1 1] Load order  : PRY
  (:Pressed
    (CallFunction|StartCustomlevelOrder (Utilities|Array|MakeArray "Level_Training" "Level_Pitch_NoMotion" "Level_Pitch" "Level_Roll_NoMotion" "Level_Roll" "Level_Yaw_NoMotion" "Level_Yaw" "Credits"))))

(event Input|KeyboardEvents|5
  (params (Key :type Key%20Structure))
  ;[1 1 1] Load order  : YPR
  (:Pressed
    (CallFunction|StartCustomlevelOrder (Utilities|Array|MakeArray "Level_Training" "Level_Pitch_NoMotion" "Level_Pitch" "Level_Roll_NoMotion" "Level_Roll" "Level_Yaw_NoMotion" "Level_Yaw" "Credits"))))

(event Input|KeyboardEvents|1
  (params (Key :type Key%20Structure))
  ;[1 1 1] Load order  : RPY
  (:Pressed
    (CallFunction|StartCustomlevelOrder (Utilities|Array|MakeArray "Level_Training" "Level_Roll_NoMotion" "Level_Roll" "Level_Pitch_NoMotion" "Level_Pitch" "Level_Yaw_NoMotion" "Level_Yaw" "Credits"))))

(event Input|KeyboardEvents|6
  (params (Key :type Key%20Structure))
  ;[1 1 1] Load order  : RYP
  (:Pressed
    (CallFunction|StartCustomlevelOrder (Utilities|Array|MakeArray "Level_Training" "Level_Roll_NoMotion" "Level_Roll" "Level_Pitch_NoMotion" "Level_Pitch" "Level_Yaw_NoMotion" "Level_Yaw" "Credits"))))

(event Input|KeyboardEvents|2
  (params (Key :type Key%20Structure))
  ;[1 1 1] Load order  : PYR
  (:Pressed
    (CallFunction|StartCustomlevelOrder (Utilities|Array|MakeArray "Level_Training" "Level_Pitch_NoMotion" "Level_Pitch" "Level_Roll_NoMotion" "Level_Roll" "Level_Yaw_NoMotion" "Level_Yaw" "Credits"))))

(event Input|KeyboardEvents|3
  (params (Key :type Key%20Structure))
  ;[1 1 1] Load order  : YPR
  (:Pressed
    (CallFunction|StartCustomlevelOrder (Utilities|Array|MakeArray "Level_Training" "Level_Pitch_NoMotion" "Level_Pitch" "Level_Roll_NoMotion" "Level_Roll" "Level_Yaw_NoMotion" "Level_Yaw" "Credits"))))

(fn ConstructionScript)

(fn StartCustomlevelOrder
  (params (LevelOrder :type Array%20of%20Names))
  (Utilities|Array|Add LevelOrder "Credits")
  (Variables|/Game/Blueprints/GI_GameInstanceCustom.GI_GameInstanceCustom_C|SetLevelsOrder (Variables|Default|GetGI) LevelOrder))