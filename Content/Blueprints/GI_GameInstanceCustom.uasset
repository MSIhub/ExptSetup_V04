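; Custom Game Instance that advances the game through an ordered list of levels.
; NextLevel increments CurrentLevel and opens that entry of LevelsOrder by name while the index is in range.
; A Gate closes on each call and reopens after a short delay, blocking repeated triggers during the transition.
; Once the index passes the last level, nothing opens and the gate stays closed.
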(event Custom|NextLevel
  (bind _levelsorder (Variables|Default|GetLevelsOrder))
  (bind _currentlevel (Variables|Default|GetCurrentLevel))
  (Utilities|FlowControl|Gate false :!label _label
    (:Exit
      (Utilities|FlowControl|Sequence
        (:then_0
          (goto _label Close))
        (:then_1
          (Math|Integer|IncrementInt _currentlevel
            (:%20%20
              (if (not (> _currentlevel (Utilities|Array|LastIndex _levelsorder)))
                (Game|OpenLevel(byName) (Utilities|Array|Get(acopy) _levelsorder _currentlevel))
                (Utilities|FlowControl|Delay 2.0)
                (goto _label Open)))))))))